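; Game mode for the front-end menu level that switches between menu screens and launches the game.
; On BeginPlay it shows the mouse cursor and displays the main menu.
; Display functions for the main, personas and weapons menus each clear all widgets, then create and add their widget to the viewport.
; StartGame opens the Game level by name.
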(event EventBeginPlay
  (Variables|/Script/Engine.PlayerController|SetbShowMouseCursor (Game|GetPlayerController 0) true)
  (CallFunction|DisplayMainMenu))

(fn ConstructionScript)

(fn DisplayPersonasMenu
  (Viewport|RemoveAllWidgets)
  (bind _returnvalue (UserInterface|CreateWidget "/Game/UI/MenuInterface/Personas/PersonasMenu_UW.PersonasMenu_UW_C"))
  (UserInterface|Viewport|AddtoViewport _returnvalue 0))

(fn DisplayMainMenu
  (Viewport|RemoveAllWidgets)
  (bind _returnvalue (UserInterface|CreateWidget "/Game/UI/MenuInterface/MainMenu_UW.MainMenu_UW_C"))
  (UserInterface|Viewport|AddtoViewport _returnvalue 0))

(fn DisplayWeaponsMenu
  (Viewport|RemoveAllWidgets)
  (bind _returnvalue (UserInterface|CreateWidget "/Game/UI/MenuInterface/Weapons/WeaponsMenu_UW.WeaponsMenu_UW_C"))
  (UserInterface|Viewport|AddtoViewport _returnvalue 0))

(fn StartGame
  (Game|OpenLevel(byName) "Game"))