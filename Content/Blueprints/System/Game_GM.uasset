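; Game mode for a survivor-style level that manages the HUD, in-game menus and end-of-run saving.
; On BeginPlay it binds the HUD to the player's components and pre-creates pause, level-up, win and lose widgets in an enum-keyed map.
; ChangeMenu toggles pause and shows or removes those widgets for level-up bonuses, wins and losses.
; ToMainMenu submits the score through the game instance's HttpManager, banks points and coins, saves, then opens Menu.
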(event EventBeginPlay
  (CallFunction|Initialization)
  (UserInterface|Viewport|AddtoViewport (Variables|Default|GetGameHUD) 0))

(event EventOnWin
  (CallFunction|ChangeMenu true false "NewEnumerator9"))

(event EventOnLoose
  (CallFunction|ChangeMenu true false "NewEnumerator10"))

(fn ConstructionScript)

(fn ToMainMenu
  (bind _asmob_survivor_gi (Utilities|Casting|CastToMobSurvivor_GI (Game|GetGameInstance)))
  (Class|HttpManager|InsertScore (Variables|/Script/ProgGameplayProto.MobSurvivorGameInstance|GetHttpManager _asmob_survivor_gi) (Variables|/Script/ProgGameplayProto.MobSurvivorSaveGame|GetPlayerToken (Variables|/Script/ProgGameplayProto.MobSurvivorGameInstance|GetSaveGameInstance _asmob_survivor_gi)) (Variables|/Script/ProgGameplayProto.CharacterData|GetName (Variables|/Script/ProgGameplayProto.MobSurvivorGameInstance|GetSelectedCharacter _asmob_survivor_gi)) (Variables|/Script/ProgGameplayProto.WeaponData|GetName (Variables|/Script/ProgGameplayProto.MobSurvivorGameInstance|GetSelectedWeapon _asmob_survivor_gi)) (Variables|/Script/ProgGameplayProto.ProjectileData|GetName (Variables|/Script/ProgGameplayProto.MobSurvivorGameInstance|GetSelectedProjectile _asmob_survivor_gi)) (Variables|Default|GetGamePoints))
  (Class|MobSurvivorGameInstance|ChangeTotalPointsby _asmob_survivor_gi (Variables|Default|GetGamePoints))
  (Class|MobSurvivorGameInstance|ChangeTotalCoinsby _asmob_survivor_gi (Variables|Default|GetGameCoins))
  (Default|SaveGame _asmob_survivor_gi)
  (Game|OpenLevel(byName) "Menu"))

(fn SetupLevelMenu
  (params (BonusNumberToDisplay :type Integer))
  (bind _menudisplayed (CallFunction|ChangeMenu true false "NewEnumerator8"))
  (bind _aslevel_up_uw (Utilities|Casting|CastToLevelUp_UW _menudisplayed))
  (Default|GetNewSetOfBonuses _aslevel_up_uw BonusNumberToDisplay))

(fn SetupHUD
  (bind _asmain_character_bp (Utilities|Casting|CastToMainCharacter_BP (Game|Player|GetPlayerPawn 0)))
  (Default|Initialize (Variables|Default|GetGameHUD) (Variables|/Script/ProgGameplayProto.MobSurvivorCharacter|GetHealth _asmain_character_bp) (Variables|/Script/ProgGameplayProto.MobSurvivorCharacter|GetExperience _asmain_character_bp) (Variables|/Script/ProgGameplayProto.MobSurvivorCharacter|GetWeapon _asmain_character_bp) (Variables|/Script/ProgGameplayProto.MobSurvivorCharacter|GetShooter _asmain_character_bp) self))

(fn Initialization
  (Variables|/Script/Engine.PlayerController|SetbShowMouseCursor (Game|GetPlayerController 0) true)
  (Utilities|FlowControl|Sequence
    (:then_0
      (bind _returnvalue (UserInterface|CreateWidget "/Game/UI/GameInterface/GameHUD_UW.GameHUD_UW_C"))
      (Variables|Default|SetGameHUD _returnvalue)
      (CallFunction|SetupHUD))
    (:then_1
      (bind _returnvalue_2 (UserInterface|CreateWidget "/Game/UI/GameInterface/PauseMenu_UW.PauseMenu_UW_C"))
      (Utilities|Map|Add (Variables|Default|GetMenus) "NewEnumerator7" _returnvalue_2))
    (:then_2
      (bind _returnvalue_3 (UserInterface|CreateWidget "/Game/UI/GameInterface/LevelUp_UW.LevelUp_UW_C"))
      (Utilities|Map|Add (Variables|Default|GetMenus) "NewEnumerator8" _returnvalue_3))
    (:then_3
      (bind _returnvalue_4 (UserInterface|CreateWidget "/Game/UI/GameInterface/WinMenu_UW.WinMenu_UW_C"))
      (Utilities|Map|Add (Variables|Default|GetMenus) "NewEnumerator9" _returnvalue_4))
    (:then_4
      (bind _returnvalue_5 (UserInterface|CreateWidget "/Game/UI/GameInterface/LooseMenu_UW.LooseMenu_UW_C"))
      (Utilities|Map|Add (Variables|Default|GetMenus) "NewEnumerator10" _returnvalue_5))))

(fn ChangeMenu
  (params (PauseGame :type Boolean) (RemoveLastMenu :type Boolean) (MenuName :type Menu_E%20Enum :default "NewEnumerator0"))
  (|RemoveLastMenu RemoveLastMenu MenuName)
  (Game|SetGamePaused PauseGame)
  (if PauseGame
    (bind _output_get (Variables|Default|SetCurrentMenu MenuName))
    (UserInterface|Viewport|AddtoViewport (.Value (Utilities|Map|Find (Variables|Default|GetMenus) _output_get)) 0)
    (return (.Value (Utilities|Map|Find (Variables|Default|GetMenus) _output_get)))))