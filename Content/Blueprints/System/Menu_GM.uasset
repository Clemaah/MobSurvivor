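; Game mode for the MobSurvivor front-end menu that creates the HUD and all menu widgets, opens on the connection screen and launches the Game level.
; Menus are pre-built into an enum-keyed map, and ChangeMenu swaps the visible one.
; Login, registration, saved-token user lookup and leaderboard requests go through the game instance's HttpManager.
; Connect updates the HUD and shows the main menu, while GetScores fills the leaderboard.
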(event EventBeginPlay
  (CallFunction|Initialization)
  (CallFunction|ChangeMenu "NewEnumerator1")
  (UserInterface|Viewport|AddtoViewport (Variables|Default|GetMenuHUD) 0)
  (CallFunction|TryGetUser))

(event EventGetScores
  (params (Scores :type Array%20of%20Score%20Object%20References))
  (CallFunction|SetUpLeaderBoard Scores))

(event EventConnect
  (params (Pseudo :type String))
  (bind _asmob_survivor_gi (Utilities|Casting|CastToMobSurvivor_GI (Game|GetGameInstance)))
  (bind _output_get (Variables|/Script/ProgGameplayProto.MobSurvivorGameInstance|SetPlayerPseudo _asmob_survivor_gi Pseudo))
  (Default|UpdateUserInfos (Variables|Default|GetMenuHUD) _output_get (Variables|/Script/ProgGameplayProto.MobSurvivorSaveGame|GetTotalCoins (Variables|/Script/ProgGameplayProto.MobSurvivorGameInstance|GetSaveGameInstance _asmob_survivor_gi)))
  (CallFunction|ChangeMenu "NewEnumerator0"))

(fn ConstructionScript)

(fn Initialization
  (Variables|/Script/Engine.PlayerController|SetbShowMouseCursor (Game|GetPlayerController 0) true)
  (Utilities|FlowControl|Sequence
    (:then_0
      (bind _returnvalue (UserInterface|CreateWidget "/Game/UI/MenuInterface/Menus/MenuHUD_UW.MenuHUD_UW_C"))
      (Variables|Default|SetMenuHUD _returnvalue))
    (:then_1
      (bind _returnvalue_2 (UserInterface|CreateWidget "/Game/UI/MenuInterface/Menus/MainMenu_UW.MainMenu_UW_C"))
      (Utilities|Map|Add (Variables|Default|GetMenus) "NewEnumerator0" _returnvalue_2))
    (:then_2
      (bind _returnvalue_3 (UserInterface|CreateWidget "/Game/UI/MenuInterface/Menus/ConnectionMenu_UW.ConnectionMenu_UW_C"))
      (Utilities|Map|Add (Variables|Default|GetMenus) "NewEnumerator1" _returnvalue_3))
    (:then_3
      (bind _returnvalue_4 (UserInterface|CreateWidget "/Game/UI/MenuInterface/Menus/RegisterMenu_UW.RegisterMenu_UW_C"))
      (Utilities|Map|Add (Variables|Default|GetMenus) "NewEnumerator2" _returnvalue_4))
    (:then_4
      (bind _returnvalue_5 (UserInterface|CreateWidget "/Game/UI/MenuInterface/Menus/LeaderBoardMenu_UW.LeaderBoardMenu_UW_C"))
      (Utilities|Map|Add (Variables|Default|GetMenus) "NewEnumerator3" _returnvalue_5))
    (:then_5
      (bind _returnvalue_6 (UserInterface|CreateWidget "/Game/UI/MenuInterface/Menus/CharactersMenu_UW.CharactersMenu_UW_C"))
      (Utilities|Map|Add (Variables|Default|GetMenus) "NewEnumerator4" _returnvalue_6))
    (:then_6
      (bind _returnvalue_7 (UserInterface|CreateWidget "/Game/UI/MenuInterface/Menus/WeaponMenu_UW.WeaponMenu_UW_C"))
      (Utilities|Map|Add (Variables|Default|GetMenus) "NewEnumerator5" _returnvalue_7))
    (:then_7
      (bind _returnvalue_8 (UserInterface|CreateWidget "/Game/UI/MenuInterface/Menus/ProjectileMenu_UW.ProjectileMenu_UW_C"))
      (Utilities|Map|Add (Variables|Default|GetMenus) "NewEnumerator6" _returnvalue_8))))

(fn ChangeMenu
  (params (MenuName :type Menu_E%20Enum :default "NewEnumerator0"))
  (Widget|RemovefromParent (.Value (Utilities|Map|Find (Variables|Default|GetMenus) (Variables|Default|GetCurrentMenu))))
  (bind _output_get (Variables|Default|SetCurrentMenu MenuName))
  (UserInterface|Viewport|AddtoViewport (.Value (Utilities|Map|Find (Variables|Default|GetMenus) _output_get)) 0)
  (return (.Value (Utilities|Map|Find (Variables|Default|GetMenus) _output_get))))

(fn TryConnection
  (params (Pseudo :type String) (Password :type String))
  (bind _asmob_survivor_gi (Utilities|Casting|CastToMobSurvivor_GI (Game|GetGameInstance)))
  (Class|HttpManager|GetToken (Variables|/Script/ProgGameplayProto.MobSurvivorGameInstance|GetHttpManager _asmob_survivor_gi) Pseudo Password))

(fn TryRegister
  (params (Email :type String) (Pseudo :type String) (Password :type String))
  (bind _asmob_survivor_gi (Utilities|Casting|CastToMobSurvivor_GI (Game|GetGameInstance)))
  (Class|HttpManager|InsertUser (Variables|/Script/ProgGameplayProto.MobSurvivorGameInstance|GetHttpManager _asmob_survivor_gi) Email Pseudo Password))

(fn TryGetUser
  (bind _asmob_survivor_gi (Utilities|Casting|CastToMobSurvivor_GI (Game|GetGameInstance)))
  (Class|HttpManager|GetUser (Variables|/Script/ProgGameplayProto.MobSurvivorGameInstance|GetHttpManager _asmob_survivor_gi) (Variables|/Script/ProgGameplayProto.MobSurvivorSaveGame|GetPlayerToken (Variables|/Script/ProgGameplayProto.MobSurvivorGameInstance|GetSaveGameInstance _asmob_survivor_gi))))

(fn TryGetScores
  (bind _asmob_survivor_gi (Utilities|Casting|CastToMobSurvivor_GI (Game|GetGameInstance)))
  (Class|HttpManager|GetLeaderBoard (Variables|/Script/ProgGameplayProto.MobSurvivorGameInstance|GetHttpManager _asmob_survivor_gi)))

(fn StartGame
  (Game|OpenLevel(byName) "Game"))

(fn SetUpLeaderBoard
  (params (Scores :type Array%20of%20Score%20Object%20References))
  (bind _menudisplayed (CallFunction|ChangeMenu "NewEnumerator3"))
  (bind _asleader_board_menu_uw (Utilities|Casting|CastToLeaderBoardMenu_UW _menudisplayed))
  (Default|SetupRankingList _asleader_board_menu_uw Scores))