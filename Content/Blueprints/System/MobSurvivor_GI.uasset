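; MobSurvivor game instance that manages selection and upgrade progression of GPEs: characters, weapons and projectiles.
; Each function switches on a type to give one generic interface over the typed data assets for selection, listing, current level and max level.
; Lists come from the save game's current-level map keys, and max level from each asset's Levels array.
; Level-ups apply to the selected item, adjust total coins by price and, like selection changes, fire notifications.
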(fn LevelUpGPE
  (params (Type :type GPE_E%20Enum :default "NewEnumerator0") (Price :type Integer))
  (switch Utilities|FlowControl|Switch|SwitchonGPE_E Type
    (:NewEnumerator0
      (Class|MobSurvivorGameInstance|LevelUpCharacter (Variables|Default|GetSelectedCharacter)))
    (:NewEnumerator1
      (Class|MobSurvivorGameInstance|LevelUpWeapon (Variables|Default|GetSelectedWeapon)))
    (:NewEnumerator2
      (Class|MobSurvivorGameInstance|LevelUpProjectile (Variables|Default|GetSelectedProjectile))))
  (bind _result (Utilities|NegateInt Price)
    (:%20%20
      (Class|MobSurvivorGameInstance|ChangeTotalCoinsby _result)
      (Default|CallOnLevelUpGPE Type))))

(fn SetSelectedGPE
  (params (GPE :type Player%20GPE%20Interface) (Type :type GPE_E%20Enum :default "NewEnumerator0"))
  (switch Utilities|FlowControl|Switch|SwitchonGPE_E Type
    (:NewEnumerator0
      (Variables|Default|SetSelectedCharacter (.AsCharacter%20Data (Utilities|Casting|CastToCharacterData GPE))))
    (:NewEnumerator1
      (Variables|Default|SetSelectedWeapon (.AsWeapon%20Data (Utilities|Casting|CastToWeaponData GPE))))
    (:NewEnumerator2
      (Variables|Default|SetSelectedProjectile (.AsProjectile%20Data (Utilities|Casting|CastToProjectileData GPE)))))
  (Default|CallOnChangeSelectedGPE GPE Type))

(fn GetGPELevel
  (params (GPE :type Player%20GPE%20Interface) (Type :type GPE_E%20Enum :default "NewEnumerator0"))
  (switch Utilities|FlowControl|Switch|SwitchonGPE_E Type
    (:NewEnumerator0
      (return (Class|MobSurvivorGameInstance|GetCharacterCurrentLevel (.AsCharacter%20Data (Utilities|Casting|CastToCharacterData GPE)))))
    (:NewEnumerator1
      (return (Class|MobSurvivorGameInstance|GetWeaponCurrentLevel (.AsWeapon%20Data (Utilities|Casting|CastToWeaponData GPE)))))
    (:NewEnumerator2
      (return (Class|MobSurvivorGameInstance|GetProjectileCurrentLevel (.AsProjectile%20Data (Utilities|Casting|CastToProjectileData GPE)))))))

(fn GetGPEList
  (params (Type :type GPE_E%20Enum :default "NewEnumerator0"))
  (switch Utilities|FlowControl|Switch|SwitchonGPE_E Type
    (:NewEnumerator0
      (bind _keys (Utilities|Map|Keys (Variables|/Script/ProgGameplayProto.MobSurvivorSaveGame|GetCharactersCurrentLevel (Variables|Default|GetSaveGameInstance))))
      (for _array_element _keys
        (Utilities|Array|Add (LocalVariables|GetList) _array_element)))
    (:NewEnumerator1
      (bind _keys_2 (Utilities|Map|Keys (Variables|/Script/ProgGameplayProto.MobSurvivorSaveGame|GetWeaponsCurrentLevel (Variables|Default|GetSaveGameInstance))))
      (for _array_element_2 _keys_2
        (Utilities|Array|Add (LocalVariables|GetList) _array_element_2)))
    (:NewEnumerator2
      (bind _keys_3 (Utilities|Map|Keys (Variables|/Script/ProgGameplayProto.MobSurvivorSaveGame|GetProjectilesCurrentLevel (Variables|Default|GetSaveGameInstance))))
      (for _array_element_3 _keys_3
        (Utilities|Array|Add (LocalVariables|GetList) _array_element_3))))
  (return (LocalVariables|GetList)))

(fn GetGPEMaxLevel
  (params (GPE :type Player%20GPE%20Interface) (Type :type GPE_E%20Enum :default "NewEnumerator0"))
  (switch Utilities|FlowControl|Switch|SwitchonGPE_E Type
    (:NewEnumerator0
      (return (- (Utilities|Array|Length (Variables|/Script/ProgGameplayProto.CharacterData|GetLevels (.AsCharacter%20Data (Utilities|Casting|CastToCharacterData GPE)))) 1)))
    (:NewEnumerator1
      (return (- (Utilities|Array|Length (Variables|/Script/ProgGameplayProto.WeaponData|GetLevels (.AsWeapon%20Data (Utilities|Casting|CastToWeaponData GPE)))) 1)))
    (:NewEnumerator2
      (return (- (Utilities|Array|Length (Variables|/Script/ProgGameplayProto.ProjectileData|GetLevels (.AsProjectile%20Data (Utilities|Casting|CastToProjectileData GPE)))) 1)))))

(fn GetSelectedGPE
  (params (Type :type GPE_E%20Enum :default "NewEnumerator0"))
  (switch Utilities|FlowControl|Switch|SwitchonGPE_E Type
    (:NewEnumerator0
      (return (Variables|Default|GetSelectedCharacter)))
    (:NewEnumerator1
      (return (Variables|Default|GetSelectedWeapon)))
    (:NewEnumerator2
      (return (Variables|Default|GetSelectedProjectile)))))