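; Game mode for the connection screen, handling player login and account registration before the main menu.
; On BeginPlay it shows the mouse cursor and displays the connection widget; separate functions swap between the connection and register widgets.
; Login and registration calls forward credentials to the HttpManager on MobSurvivor_GI to get a token or insert a user.
; The Connect event checks the game instance type and opens the Menu level.
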(event EventBeginPlay
  (Variables|/Script/Engine.PlayerController|SetbShowMouseCursor (Game|GetPlayerController 0) true)
  (CallFunction|DisplayConnectionMenu))

(event EventConnect
  (params (Pseudo :type String))
  (Utilities|Casting|CastToMobSurvivor_GI (Game|GetGameInstance))
  (Game|OpenLevel(byName) "Menu"))

(fn ConstructionScript)

(fn DisplayConnectionMenu
  (Viewport|RemoveAllWidgets)
  (bind _returnvalue (UserInterface|CreateWidget "/Game/UI/ConnectionInterface/ConnectionMenu_UW.ConnectionMenu_UW_C"))
  (UserInterface|Viewport|AddtoViewport _returnvalue 0))

(fn DisplayRegisterMenu
  (Viewport|RemoveAllWidgets)
  (bind _returnvalue (UserInterface|CreateWidget "/Game/UI/ConnectionInterface/RegisterMenu_UW.RegisterMenu_UW_C"))
  (UserInterface|Viewport|AddtoViewport _returnvalue 0))

(fn TryConnection
  (params (Pseudo :type String) (Password :type String))
  (bind _asmob_survivor_gi (Utilities|Casting|CastToMobSurvivor_GI (Game|GetGameInstance)))
  (Class|HttpManager|GetToken (Variables|/Script/ProgGameplayProto.MobSurvivorGameInstance|GetHttpManager _asmob_survivor_gi) Pseudo Password))

(fn TryRegister
  (params (Email :type String) (Pseudo :type String) (Password :type String))
  (bind _asmob_survivor_gi (Utilities|Casting|CastToMobSurvivor_GI (Game|GetGameInstance)))
  (Class|HttpManager|InsertUser (Variables|/Script/ProgGameplayProto.MobSurvivorGameInstance|GetHttpManager _asmob_survivor_gi) Email Pseudo Password))