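; Game mode for the menu level that switches between the main, weapons, characters and projectiles menu screens.
; On BeginPlay it shows the mouse cursor and opens the main menu.
; Each display function clears all widgets, then creates its menu widget and adds it to the viewport, so one screen shows at a time.
; StartGame opens the "Game" level.
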(event EventBeginPlay
  (Variables|/Script/Engine.PlayerController|SetbShowMouseCursor (Game|GetPlayerController 0) true)
  (CallFunction|DisplayMainMenu))

(fn ConstructionScript)

(fn StartGame
  (Game|OpenLevel(byName) "Game"))

(fn DisplayWeaponsMenu
  (Viewport|RemoveAllWidgets)
  (bind _returnvalue (UserInterface|CreateWidget "/Game/UI/MenuInterface/Weapons/WeaponsMenu_UW.WeaponsMenu_UW_C"))
  (UserInterface|Viewport|AddtoViewport _returnvalue 0))

(fn DisplayMainMenu
  (Viewport|RemoveAllWidgets)
  (bind _returnvalue (UserInterface|CreateWidget "/Game/UI/MenuInterface/MainMenu_UW.MainMenu_UW_C"))
  (UserInterface|Viewport|AddtoViewport _returnvalue 0))

(fn DisplayCharactersMenu
  (Viewport|RemoveAllWidgets)
  (bind _returnvalue (UserInterface|CreateWidget "/Game/UI/MenuInterface/Characters/CharacterMenu_UW.CharacterMenu_UW_C"))
  (UserInterface|Viewport|AddtoViewport _returnvalue 0))

(fn DisplayProjectilesMenu
  (Viewport|RemoveAllWidgets)
  (bind _returnvalue (UserInterface|CreateWidget "/Game/UI/MenuInterface/Projectiles/ProjectilesMenu_UW.ProjectilesMenu_UW_C"))
  (UserInterface|Viewport|AddtoViewport _returnvalue 0))