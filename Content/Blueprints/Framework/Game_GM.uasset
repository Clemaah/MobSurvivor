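; Game mode for the survivor game that handles pausing, in-game menus and returning to the main menu.
; Level-up and pause functions pause the game and add their widgets to the viewport, with the level-up widget also requesting a new set of bonuses.
; Resuming unpauses and removes all widgets.
; Leaving saves through the MobSurvivor game instance, then opens the Menu level.
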(event EventBeginPlay)

(event EventTick
  (params (DeltaSeconds :type Float%20%28single-precision%29)))

(fn ConstructionScript)

(fn ResumeGame
  (Game|SetGamePaused false)
  (Viewport|RemoveAllWidgets))

(fn ToMainMenu
  (bind _asmob_survivor_gi (Utilities|Casting|CastToMobSurvivor_GI (Game|GetGameInstance)))
  (Class|MobSurvivorGameInstance|SaveGame _asmob_survivor_gi)
  (Game|OpenLevel(byName) "Menu"))

(fn DisplayLevelMenu
  (Game|SetGamePaused true)
  (bind _returnvalue (UserInterface|CreateWidget "/Game/UI/GameInterface/LevelUp_UW.LevelUp_UW_C"))
  (UserInterface|Viewport|AddtoViewport _returnvalue 0)
  (Default|GetNewSetOfBonuses _returnvalue))

(fn DisplayPauseMenu
  (Game|SetGamePaused true)
  (bind _returnvalue (UserInterface|CreateWidget "/Game/UI/GameInterface/PauseMenu_UW.PauseMenu_UW_C"))
  (UserInterface|Viewport|AddtoViewport _returnvalue 0))