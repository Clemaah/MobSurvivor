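; Player character Blueprint for a mob-survivor game, configured from the selected character, weapon and projectile.
; On BeginPlay it reads their level-based characteristics from the game instance and passes them to SetupComponents.
; Experience level-ups open the level menu through the game mode, and the pause input switches menus.
; Low health drives a damage vignette through a material parameter collection, scaling as health drops below a threshold.
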(event Custom|OnLevelUp
  (params (NewLevel :type Integer) (NewXpTarget :type Float%20%28double-precision%29))
  (bind _asgame_gm (Utilities|Casting|CastToGame_GM (Game|GetGameMode)))
  (Default|SetupLevelMenu _asgame_gm))

(event Custom|UpdateHealthPostProcess
  (params (Health :type Float%20%28double-precision%29))
  (bind _healthlevelforstartvignetteshowing (Variables|Default|GetHealthLevelForStartVignetteShowing))
  (if (< Health _healthlevelforstartvignetteshowing)
    (Rendering|Material|SetScalarParameterValue "/Game/VFX/MPC_Vignette.MPC_Vignette" "DamageLevel" (- 1.0 (/ Health _healthlevelforstartvignetteshowing)) :!class /Script/Engine.KismetMaterialLibrary)
    (else
      (Rendering|Material|SetScalarParameterValue "/Game/VFX/MPC_Vignette.MPC_Vignette" "DamageLevel" 0.0 :!class /Script/Engine.KismetMaterialLibrary))))

(event Input|EnhancedActionEvents|EnhancedInputActionIA_Pause
  (params (ActionValue :type Boolean) (ElapsedSeconds :type Float%20%28double-precision%29) (TriggeredSeconds :type Float%20%28double-precision%29) (InputAction :type Input%20Action%20Object%20Reference :default "/Game/Input/Actions/IA_Pause.IA_Pause"))
  (bind _asgame_gm (Utilities|Casting|CastToGame_GM (Game|GetGameMode)))
  (Default|ChangeMenu _asgame_gm true false "NewEnumerator7"))

(event EventBeginPlay
  (CallFunction|SetupCharacter)
  (EventDispatchers|BindEventtoOnLevelUp (Variables|Default|GetExperience) (EventDispatchers|CreateEvent :!event Custom|OnLevelUp)))

(fn ConstructionScript)

(fn SetupCharacter
  (bind _asmob_survivor_gi (Utilities|Casting|CastToMobSurvivor_GI (Game|GetGameInstance)))
  (bind _returnvalue (Class|ProjectileData|GetCurrentCharacteristics (Variables|/Script/ProgGameplayProto.MobSurvivorGameInstance|GetSelectedProjectile _asmob_survivor_gi) (Class|MobSurvivorGameInstance|GetProjectileCurrentLevel _asmob_survivor_gi (Variables|/Script/ProgGameplayProto.MobSurvivorGameInstance|GetSelectedProjectile _asmob_survivor_gi))))
  (bind _returnvalue_2 (Class|WeaponData|GetCurrentCharacteristics (Variables|/Script/ProgGameplayProto.MobSurvivorGameInstance|GetSelectedWeapon _asmob_survivor_gi) (Class|MobSurvivorGameInstance|GetWeaponCurrentLevel _asmob_survivor_gi (Variables|/Script/ProgGameplayProto.MobSurvivorGameInstance|GetSelectedWeapon _asmob_survivor_gi))))
  (bind _returnvalue_3 (Class|CharacterData|GetCurrentCharacterCharacteristics (Variables|/Script/ProgGameplayProto.MobSurvivorGameInstance|GetSelectedCharacter _asmob_survivor_gi) (Class|MobSurvivorGameInstance|GetCharacterCurrentLevel _asmob_survivor_gi (Variables|/Script/ProgGameplayProto.MobSurvivorGameInstance|GetSelectedCharacter _asmob_survivor_gi))))
  (bind _returnvalue_4 (Class|CharacterData|GetCurrentPersonaCharacteristics (Variables|/Script/ProgGameplayProto.MobSurvivorGameInstance|GetSelectedCharacter _asmob_survivor_gi) (Class|MobSurvivorGameInstance|GetCharacterCurrentLevel _asmob_survivor_gi (Variables|/Script/ProgGameplayProto.MobSurvivorGameInstance|GetSelectedCharacter _asmob_survivor_gi))))
  (Class|MobSurvivorCharacter|SetupComponents _returnvalue_4 _returnvalue_3 _returnvalue_2 _returnvalue (Variables|/Script/ProgGameplayProto.ProjectileData|GetProjectileToSpawn (Variables|/Script/ProgGameplayProto.MobSurvivorGameInstance|GetSelectedProjectile _asmob_survivor_gi)) (Variables|/Script/ProgGameplayProto.ProjectileData|GetEffects (Variables|/Script/ProgGameplayProto.MobSurvivorGameInstance|GetSelectedProjectile _asmob_survivor_gi))))