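; HealDrop is a drop actor, named as a healing pickup, whose graph contains only its idle spin and bob animation.
; Each Tick adds a delta-time-scaled yaw to the Cube component from its world rotation, zeroing pitch and roll.
; It also sets the Cube's relative Z from a sine of game time to make it hover.
; No healing or overlap logic is implemented in this graph.
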(event EventBeginPlay)

(event Collision|EventActorBeginOverlap
  (params (OtherActor :type Actor%20Object%20Reference)))

(event EventTick
  (params (DeltaSeconds :type Float%20%28single-precision%29))
  (bind _cube (Variables|Default|GetCube))
  (Transformation|SetRelativeRotation _cube (Math|Rotator|MakeRotator 0.0 0.0 (+ (.yaw (Transformation|GetWorldRotation (Variables|Default|GetCube))) (* DeltaSeconds 5e+01))) false false)
  (Transformation|SetRelativeLocation _cube (Math|Vector|MakeVector 0.0 0.0 (* (Math|Trig|Sin(Radians) (* (Utilities|Time|GetTimeSeconds) 3.0)) 1e+01)) false false))

(fn ConstructionScript)