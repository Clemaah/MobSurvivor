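; Chest pickup that animates its lid open and, when collected, brings up the level menu with a set number of bonuses to choose.
; While in the Opening state, Tick linearly pitches the Top component toward the opening angle over a set duration, then switches to Open and activates a Niagara effect.
; OnCollect asks Game_GM to set up that menu; the trigger for the Opening state is not in this graph.
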(event EventTick
  (params (DeltaSeconds :type Float%20%28single-precision%29))
  (if (Utilities|Enum|Equal(Enum) (Variables|Default|GetState) "Opening")
    (bind _output_get (Variables|Default|SetOpeningElapsedTime (+ DeltaSeconds (Variables|Default|GetOpeningElapsedTime))))
    (Transformation|SetRelativeRotation (Variables|Default|GetTop) (Math|Rotator|MakeRotator 0.0 (* (/ _output_get (Variables|Default|GetOpeningDuration)) (Variables|Default|GetOpeningAngle)) 0.0) false false)
    (if (>= (Variables|Default|GetOpeningElapsedTime) (Variables|Default|GetOpeningDuration))
      (Variables|Default|SetState "Open")
      (Components|Activation|Activate (Variables|Default|GetNiagara) false))))

(event EventOnCollect
  (bind _asgame_gm (Utilities|Casting|CastToGame_GM (Game|GetGameMode)))
  (Default|SetupLevelMenu _asgame_gm (Variables|Default|GetBonusNumberToChoose)))

(fn ConstructionScript)